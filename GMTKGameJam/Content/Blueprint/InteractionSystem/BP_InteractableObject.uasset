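; Base interactable world object that supplies a dialogue row name on interaction and can grant a key once or hide itself.
; The game instance's day-change event selects the row from a day-to-row map by index.
; Interact registers it as the current object, firing finished-dialogue when switching objects, and blocks repeats until that event resets it.
; It also exposes hover and click crosshair textures and sets its mesh at construction.
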(event Custom|OnDayChange_Event
  (Variables|Default|SetRowName (.Value (Utilities|Map|GetKeyValueByIndex (Variables|Config|GetDayToRowName) (Variables|/Game/Blueprint/GI_Main.GI_Main_C|GetCurrentDay (CallFunction|GetCurrentGameInstance))))))

(event Custom|ResetObject
  (Variables|Default|SetbIsAlreadyInteracting false))

(event EventBeginPlay
  (Variables|Default|SetTags (Variables|Config|GetLevelTag))
  (EventDispatchers|AssignOnDayChange (CallFunction|GetCurrentGameInstance) (delegate Custom|OnDayChange_Event))
  (Variables|Default|SetCrosshairToSet (Variables|Crosshair|GetCrosshairHover))
  (EventDispatchers|BindEventtoFinishedDialogue (CallFunction|GetCurrentGameInstance) (delegate Custom|ResetObject)))

(event EventSetClickCrosshair
  (CallFunction|UpdateCrosshairtoSet (Variables|Crosshair|GetCrosshairClick)))

(event EventResetCrosshair
  (CallFunction|UpdateCrosshairtoSet (Variables|Crosshair|GetCrosshairHover)))

(fn ConstructionScript
  (Components|StaticMesh|SetStaticMesh (Variables|Default|GetMesh) (Variables|Config|GetMeshToSet)))

(fn HideObject
  (Rendering|SetActorHiddenInGame true)
  (Collision|SetActorEnableCollision false))

(fn UpdateCrosshairtoSet
  (params (CrosshairTexture :type Texture%202D%20Object%20Reference))
  (Variables|Default|SetCrosshairToSet CrosshairTexture))

(fn GetCursorImage
  (return (Variables|Default|GetCrosshairToSet)))

(fn Interact
  (bind _gi_main (CallFunction|GetCurrentGameInstance))
  (if (!= self (Variables|/Game/Blueprint/GI_Main.GI_Main_C|GetCurrentInteractionObj _gi_main))
    (Default|CallFinishedDialogue _gi_main))
  (Variables|/Game/Blueprint/GI_Main.GI_Main_C|SetCurrentInteractionObj _gi_main self)
  (Variables|Default|GetbIsAlreadyInteracting
    (:then)
    (:else
      (Variables|Default|SetbIsAlreadyInteracting true)
      (Variables|Config|GetbCanGiveButton
        (:then
          (Default|CallAddKey (CallFunction|GetCurrentGameInstance))
          (Variables|Config|SetbCanGiveButton false)
          (Variables|Config|GetbHasToDisappear
            (:then
              (CallFunction|HideObject))
            (:else
              _))
          (return (Variables|Default|GetRowName)))
        (:else
          (Variables|Config|GetbHasToDisappear
            (:then
              (CallFunction|HideObject))
            (:else
              _))
          (return (Variables|Default|GetRowName)))))))