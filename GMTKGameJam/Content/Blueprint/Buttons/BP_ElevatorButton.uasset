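; Interactable elevator button that animates into its plate and, when pressed, starts the elevator.
; At BeginPlay it registers event delegates with the game instance, then reveals itself and slides in along world X via a timeline.
; Interact is guarded for a single press, returning a row name and playing a press timeline that calls the game instance's start-elevator function on finish.
; It also supplies hover or click crosshair images and can be repositioned through AttachToElevator.
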(event Custom|InsertButton
  (bind _returnvalue (Transformation|GetActorLocation))
  (Variables|Default|GetBIsInsert
    (:then)
    (:else
      (Variables|Default|SetBIsInsert true)
      (Variables|Default|SetCorrectLocation (Math|Vector|MakeVector (.x _returnvalue) (.y _returnvalue) (.z _returnvalue)))
      (Transformation|SetActorLocation (Math|Vector|MakeVector (+ (.x _returnvalue) (Variables|Default|GetDistanceFromPlate)) (.y _returnvalue) (.z _returnvalue)) false true)
      (Rendering|SetActorHiddenInGame false)
      (bind _delta (Timeline|InsertTimeline PlayFromStart)
        (:Update
          (Transformation|SetActorLocation (Math|Vector|MakeVector (Math|Float|Lerp (+ (.x (Variables|Default|GetCorrectLocation)) 5.0) (.x (Variables|Default|GetCorrectLocation)) _delta) (.y (Variables|Default|GetCorrectLocation)) (.z (Variables|Default|GetCorrectLocation))) false false)
          (Collision|SetActorEnableCollision true))))))

(event Custom|PressButton
  (bind _correctlocation (Variables|Default|GetCorrectLocation))
  (bind _delta (Timeline|PressTimeline PlayFromStart)
    (:Update
      (Transformation|SetActorLocation (Math|Vector|MakeVector (Math|Float|Lerp (.x _correctlocation) (- (.x _correctlocation) 2.0) _delta) (.y _correctlocation) (.z _correctlocation)) false false))
    (:Finished
      (Default|CallStartElevator (CallFunction|GetCurrentGameInstance)))))

(event Custom|AttachToElevator
  (params (Position :type Vector))
  (Transformation|SetActorLocation Position false false))

(event EventBeginPlay
  (bind _gi_main (CallFunction|GetCurrentGameInstance))
  (Variables|Default|SetBIsInsert false)
  (Variables|Default|SetbAlreadyPressed false)
  (Rendering|SetActorHiddenInGame true)
  (Collision|SetActorEnableCollision false)
  (Variables|Default|SetImageToSet (Variables|Default|GetHoverImage))
  (EventDispatchers|AssignAttachItems _gi_main (EventDispatchers|CreateEvent :!event Custom|AttachToElevator))
  (EventDispatchers|AssignAttachButton _gi_main (EventDispatchers|CreateEvent :!event Custom|InsertButton))
  (CallFunction|InsertButton))

(event EventResetCrosshair
  (Variables|Default|SetImageToSet (Variables|Default|GetHoverImage)))

(event EventSetClickCrosshair
  (Variables|Default|SetImageToSet (Variables|Default|GetClickImage)))

(fn ConstructionScript)

(fn GetCursorImage
  (return (Variables|Default|GetImageToSet)))

(fn Interact
  (Variables|Default|GetbAlreadyPressed
    (:then)
    (:else
      (Variables|Default|SetbAlreadyPressed true)
      (CallFunction|PressButton)
      (return (Variables|Default|GetRowName)))))