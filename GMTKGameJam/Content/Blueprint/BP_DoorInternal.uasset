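; Interior door actor that swings open on DoorInteract and closes itself after a delay.
; DoorRotation plays a timeline that lerps Door1's absolute world yaw from zero to DoorRotationValue.
; When opening finishes, AutoClose reverses the same timeline after TimeBeforeClose.
; The IsOpen flag gates interaction and keeps the closing pass from retriggering the delay; the Interact function only returns None.
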(event Custom|DoorRotation
  (Variables|Default|SetbIsOpen true)
  (bind _delta (Timeline|Timeline PlayFromStart)
    (:Update
      (Transformation|SetWorldRotation (Variables|Default|Getdoor1) (Math|Rotator|MakeRotator 0.0 0.0 (Math|Float|Lerp 0.0 (Variables|Default|GetDoorRotationValue) _delta)) false false))
    (:Finished
      (Variables|Default|GetbIsOpen
        (:then
          (Variables|Default|SetbIsOpening false)
          (Utilities|FlowControl|Delay (Variables|Default|GetTimeBeforeClose))
          (CallFunction|AutoClose))
        (:else)))))

(event Custom|AutoClose
  (Variables|Default|SetbIsOpen false)
  (bind _delta (Timeline|Timeline ReverseFromEnd)
    (:Update
      (Transformation|SetWorldRotation (Variables|Default|Getdoor1) (Math|Rotator|MakeRotator 0.0 0.0 (Math|Float|Lerp 0.0 (Variables|Default|GetDoorRotationValue) _delta)) false false))
    (:Finished
      (Variables|Default|GetbIsOpen
        (:then
          (Variables|Default|SetbIsOpening false)
          (Utilities|FlowControl|Delay (Variables|Default|GetTimeBeforeClose))
          (CallFunction|AutoClose))
        (:else)))))

(event EventDoorInteract
  (Variables|Default|GetbIsOpen
    (:then)
    (:else
      (Variables|Default|SetbIsOpening false)
      (CallFunction|DoorRotation))))

(fn ConstructionScript)

(fn Interact
  (return "None"))