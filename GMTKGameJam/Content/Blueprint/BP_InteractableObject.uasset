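; Interactable world object that returns a row name when interacted with, varying by the current day.
; On the game instance's day change it picks the row from a day-to-row map, using the current day as index.
; Interact can grant a key once through the game instance, and optionally hides the object and disables its collision before returning the row.
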(event Custom|OnDayChange_Event
  (Variables|Default|SetRowName (.Value (Utilities|Map|GetKeyValueByIndex (Variables|Default|GetDayToRowName) (Variables|/Game/Blueprint/GI_Main.GI_Main_C|GetCurrentDay (CallFunction|GetCurrentGameInstance))))))

(event EventBeginPlay
  (Variables|Default|SetTags (Variables|Default|GetLevelTag))
  (EventDispatchers|AssignOnDayChange (CallFunction|GetCurrentGameInstance) (delegate Custom|OnDayChange_Event)))

(fn ConstructionScript)

(fn HideObject
  (Rendering|SetActorHiddenInGame true)
  (Collision|SetActorEnableCollision false))

(fn Interact
  (Variables|Default|GetbCanGiveButton
    (:then
      (Default|CallAddKey (CallFunction|GetCurrentGameInstance))
      (Variables|Default|SetbCanGiveButton false)
      (Variables|Default|GetbHasToDisappear
        (:then
          (CallFunction|HideObject))
        (:else
          _))
      (return (Variables|Default|GetRowName)))
    (:else
      (Variables|Default|GetbHasToDisappear
        (:then
          (CallFunction|HideObject))
        (:else
          _))
      (return (Variables|Default|GetRowName)))))