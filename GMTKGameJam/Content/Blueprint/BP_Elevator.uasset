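; Elevator actor that starts with its swing doors open and runs a ride when the game instance signals a start.
; Move closes the doors with a timeline, then a second timeline slides the car by a vertical offset.
; At the end it attaches the player, snaps the car back to its origin, detaches and signals finish through the game instance.
; OpenDoor reverses the door timeline, clearing IsDescending, the flag meant to gate the ride.
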(event Custom|Move
  (bind _sm_elevatorrightdoor1 (Variables|Default|GetSM_ElevatorRightDoor1))
  (bind _sm_elevatorleftdoor1 (Variables|Default|GetSM_ElevatorLeftDoor1))
  (bind _relativerotation (Variables|/Script/Engine.SceneComponent|GetRelativeRotation _sm_elevatorrightdoor1))
  (bind _relativerotation_2 (Variables|/Script/Engine.SceneComponent|GetRelativeRotation _sm_elevatorleftdoor1))
  (Variables|Default|SetbIsDescending true)
  (bind _alpha (Timeline|DoorOpenClose PlayFromStart)
    (:Update
      (Utilities|FlowControl|Sequence
        (:then_0
          (Transformation|SetRelativeRotation (Variables|Default|GetSM_ElevatorRightDoor1) (Math|Rotator|MakeRotator (.roll _relativerotation) (.pitch _relativerotation) (Math|Float|Lerp (Variables|Default|GetOpenZRightDoor) (Variables|Default|GetRightDefaultZ) _alpha)) false false))
        (:then_1
          (Transformation|SetRelativeRotation (Variables|Default|GetSM_ElevatorLeftDoor1) (Math|Rotator|MakeRotator (.roll _relativerotation_2) (.pitch _relativerotation_2) (Math|Float|Lerp (Variables|Default|GetOpenZLeftDoor) (Variables|Default|GetLeftDefaultZ) _alpha)) false false))))
    (:Finished
      (Variables|Default|GetbIsDescending
        (:then
          (Utilities|FlowControl|Delay 0.1)
          (bind _alpha_2 (Timeline|ElevatorMovement PlayFromStart)
            (:Update
              (Transformation|SetRelativeLocation (Variables|Default|GetElevator) (Math|Vector|Lerp(Vector) "0, 0, 0" (Variables|Default|GetTeleportLoc) _alpha_2) true false))
            (:Finished
              (Default|CallAttachPlayer self)
              (Transformation|SetRelativeLocation (Variables|Default|GetElevator) "0, 0, 0" false true)
              (Default|CallDetachPlayer)
              (Default|CallElevatorFinish (CallFunction|GetCurrentGameInstance)))))
        (:else)))))

(event Custom|OpenDoor
  (bind _sm_elevatorrightdoor1 (Variables|Default|GetSM_ElevatorRightDoor1))
  (bind _sm_elevatorleftdoor1 (Variables|Default|GetSM_ElevatorLeftDoor1))
  (bind _relativerotation (Variables|/Script/Engine.SceneComponent|GetRelativeRotation _sm_elevatorrightdoor1))
  (bind _relativerotation_2 (Variables|/Script/Engine.SceneComponent|GetRelativeRotation _sm_elevatorleftdoor1))
  (Variables|Default|SetbIsDescending false)
  (bind _alpha (Timeline|DoorOpenClose ReverseFromEnd)
    (:Update
      (Utilities|FlowControl|Sequence
        (:then_0
          (Transformation|SetRelativeRotation (Variables|Default|GetSM_ElevatorRightDoor1) (Math|Rotator|MakeRotator (.roll _relativerotation) (.pitch _relativerotation) (Math|Float|Lerp (Variables|Default|GetOpenZRightDoor) (Variables|Default|GetRightDefaultZ) _alpha)) false false))
        (:then_1
          (Transformation|SetRelativeRotation (Variables|Default|GetSM_ElevatorLeftDoor1) (Math|Rotator|MakeRotator (.roll _relativerotation_2) (.pitch _relativerotation_2) (Math|Float|Lerp (Variables|Default|GetOpenZLeftDoor) (Variables|Default|GetLeftDefaultZ) _alpha)) false false))))
    (:Finished
      (Variables|Default|GetbIsDescending
        (:then
          (Utilities|FlowControl|Delay 0.1)
          (bind _alpha_2 (Timeline|ElevatorMovement PlayFromStart)
            (:Update
              (Transformation|SetRelativeLocation (Variables|Default|GetElevator) (Math|Vector|Lerp(Vector) "0, 0, 0" (Variables|Default|GetTeleportLoc) _alpha_2) true false))
            (:Finished
              (Default|CallAttachPlayer self)
              (Transformation|SetRelativeLocation (Variables|Default|GetElevator) "0, 0, 0" false true)
              (Default|CallDetachPlayer)
              (Default|CallElevatorFinish (CallFunction|GetCurrentGameInstance)))))
        (:else)))))

(event EventBeginPlay
  (bind _sm_elevatorrightdoor1 (Variables|Default|GetSM_ElevatorRightDoor1))
  (bind _sm_elevatorleftdoor1 (Variables|Default|GetSM_ElevatorLeftDoor1))
  (bind _relativerotation (Variables|/Script/Engine.SceneComponent|GetRelativeRotation _sm_elevatorleftdoor1))
  (bind _relativerotation_2 (Variables|/Script/Engine.SceneComponent|GetRelativeRotation _sm_elevatorrightdoor1))
  (Variables|Default|SetTeleportLoc (Math|Vector|MakeVector 0.0 0.0 (Variables|Default|GetVertical%20Offset)))
  (EventDispatchers|BindEventtoStartElevator (CallFunction|GetCurrentGameInstance) (delegate Custom|Move))
  (EventDispatchers|BindEventtoElevatorFinish (CallFunction|GetCurrentGameInstance) (EventDispatchers|CreateEvent :!event Custom|OpenDoor))
  (Variables|Default|SetRightDefaultZ (.roll (Variables|/Script/Engine.SceneComponent|GetRelativeRotation (Variables|Default|GetSM_ElevatorRightDoor1))))
  (Variables|Default|SetLeftDefaultZ (.roll (Variables|/Script/Engine.SceneComponent|GetRelativeRotation (Variables|Default|GetSM_ElevatorLeftDoor1))))
  (bind _output_get (Variables|Default|SetOpenZLeftDoor (+ (.yaw _relativerotation) 1.5e+02)))
  (Transformation|SetRelativeRotation _sm_elevatorleftdoor1 (Math|Rotator|MakeRotator (.roll _relativerotation) (.pitch _relativerotation) _output_get) false false)
  (bind _output_get_2 (Variables|Default|SetOpenZRightDoor (- (.yaw _relativerotation_2) 1.5e+02)))
  (Transformation|SetRelativeRotation _sm_elevatorrightdoor1 (Math|Rotator|MakeRotator (.roll _relativerotation_2) (.pitch _relativerotation_2) _output_get_2) false false))

(fn ConstructionScript)