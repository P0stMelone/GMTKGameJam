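; Interactable door that swings Door1 open and closes itself automatically after a delay.
; DoorInteract checks the lock, plays an optional sound and, if closed, runs a Timeline that lerps the yaw, later reversing it.
; Interact only registers the door as the game instance's current interaction object.
; GetCursorImage returns the hover or click crosshair, which separate events switch between.
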(event Custom|DoorRotation
  (Variables|Default|SetbIsOpen true)
  (bind _delta (Timeline|Timeline PlayFromStart)
    (:Update
      (Transformation|SetRelativeRotation (Variables|Default|Getdoor1) (Math|Rotator|MakeRotator 0.0 0.0 (Math|Float|Lerp 0.0 (Variables|Default|GetDoorRotationValue) _delta)) false false))
    (:Finished
      (Variables|Default|GetbIsOpen
        (:then
          (Variables|Default|SetbIsOpening false)
          (Utilities|FlowControl|Delay (Variables|Default|GetTimeBeforeClose))
          (CallFunction|AutoClose))
        (:else)))))

(event Custom|AutoClose
  (Variables|Default|SetbIsOpen false)
  (bind _delta (Timeline|Timeline ReverseFromEnd)
    (:Update
      (Transformation|SetRelativeRotation (Variables|Default|Getdoor1) (Math|Rotator|MakeRotator 0.0 0.0 (Math|Float|Lerp 0.0 (Variables|Default|GetDoorRotationValue) _delta)) false false))
    (:Finished
      (Variables|Default|GetbIsOpen
        (:then
          (Variables|Default|SetbIsOpening false)
          (Utilities|FlowControl|Delay (Variables|Default|GetTimeBeforeClose))
          (CallFunction|AutoClose))
        (:else)))))

(event EventResetCrosshair
  (Variables|Default|SetCrosshairToSet (Variables|Default|GetHoverCrosshair)))

(event EventSetClickCrosshair
  (Variables|Default|SetCrosshairToSet (Variables|Default|GetClickCrosshair)))

(event EventDoorInteract
  (bind _soundtoreproduce (Variables|Default|GetSoundToReproduce))
  (Variables|Default|GetbIsLocked
    (:then)
    (:else
      (Utilities|IsValid _soundtoreproduce
        (:Is%20Valid
          (Audio|PlaySoundatLocation _soundtoreproduce (Transformation|GetActorLocation) "0, 0, 0" 1.0 1.0 0.0 0 0 0 0))
        (:Is%20Not%20Valid
          _))
      (Variables|Default|GetbIsOpen
        (:then)
        (:else
          (Variables|Default|SetbIsOpening false)
          (CallFunction|DoorRotation))))))

(event EventBeginPlay
  (Variables|Default|SetCrosshairToSet (Variables|Default|GetHoverCrosshair)))

(fn ConstructionScript)

(fn GetCursorImage
  (return (Variables|Default|GetCrosshairToSet)))

(fn Interact
  (Variables|/Game/Blueprint/GI_Main.GI_Main_C|SetCurrentInteractionObj (CallFunction|GetCurrentGameInstance) self)
  (return "None"))