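; Dialogue component that steps through lines of text stored in the DT_Dialogues data table.
; StartDialogue plays a given row, and NextLine follows that row's NextRowName like a linked list.
; It broadcasts each line's text through OnDialogueUpdate and fires OnDialogueEnded at a chain's end or when the row to play is missing.
; On BeginPlay it binds to the game instance's finished-dialogue event, allowing a forced end.
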(event Custom|ForcedEnd
  (Default|CallOnDialogueEnded))

(event EventBeginPlay
  (EventDispatchers|BindEventtoFinishedDialogue (CallFunction|GetCurrentGameInstance) (delegate Custom|ForcedEnd)))

(fn StartDialogue
  (params (RowName :type Name))
  (Variables|Default|SetCurrentRowName RowName)
  (CallFunction|PlayCurrentLine))

(fn PlayCurrentLine
  (bind _returnvalue (Utilities|GetDataTableRow "/Game/Blueprint/DialogueSystem/DT_Dialogues.DT_Dialogues" (Variables|Default|GetCurrentRowName))
    (:then
      (Default|CallOnDialogueUpdate (.DialogueText (Utilities|Struct|BreakF_DialogueLine _returnvalue))))
    (:RowNotFound
      (Default|CallOnDialogueEnded))))

(fn NextLine
  (bind _returnvalue (Utilities|GetDataTableRow "/Game/Blueprint/DialogueSystem/DT_Dialogues.DT_Dialogues" (Variables|Default|GetCurrentRowName))
    (:then
      (if (!= (.NextRowName (Utilities|Struct|BreakF_DialogueLine _returnvalue)) "")
        (Variables|Default|SetCurrentRowName (.NextRowName (Utilities|Struct|BreakF_DialogueLine _returnvalue)))
        (CallFunction|PlayCurrentLine)
        (else
          (Default|CallOnDialogueEnded))))))