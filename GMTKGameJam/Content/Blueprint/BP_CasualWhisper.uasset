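; BP_CasualWhisper is an ambient audio Blueprint that layers a one-off whispering-trees sound over background brown noise.
; On BeginPlay it picks a random delay and starts the brown noise as a 2D sound.
; After the delay, ReproduceSound plays the whisper at the player pawn's location.
; Nothing re-triggers the delay, so the whisper fires only once per BeginPlay.
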(event Custom|SetDelayTime
  (Variables|Default|SetDelayTime (Math|Random|RandomFloatinRange 2e+01 5e+01))
  (CallFunction|ReproduceSound))

(event Custom|ReproduceSound
  (Utilities|FlowControl|Delay (Variables|Default|GetDelayTime))
  (Audio|PlaySoundatLocation "/Game/Art/Sound/Whispers/CasualWhispert/freesound_community-whispering-trees-35410.freesound_community-whispering-trees-35410" (Transformation|GetActorLocation (Game|Player|GetPlayerPawn 0)) "0, 0, 0" 0.8 1.0 0.0 0 0 0 0))

(event EventBeginPlay
  (CallFunction|SetDelayTime)
  (Audio|SpawnSound2D "/Game/Art/Sound/BrownNoiseBackground.BrownNoiseBackground" 0.5 1.0 0.0 0))

(fn ConstructionScript)