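; BP_Pulsantiera is an interactable button panel that a key lets the player attach to the elevator.
; Interact checks the game instance's HasKey, then either fires the RemoveKey and AttachButton dispatchers or returns a "MissingKey" row name.
; On BeginPlay it binds to the game instance's AttachItems dispatcher, with AttachToElevator moving the actor to a supplied position.
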(event Custom|AttachToElevator
  (params (Position :type Vector))
  (Transformation|SetActorLocation Position false false))

(event EventBeginPlay
  (EventDispatchers|AssignAttachItems (CallFunction|GetCurrentGameInstance) (EventDispatchers|CreateEvent :!event Custom|AttachToElevator)))

(fn ConstructionScript)

(fn GetCursorImage
  (return 0))

(fn Interact
  (bind _gi_main (CallFunction|GetCurrentGameInstance))
  (Variables|/Game/Blueprint/GI_Main.GI_Main_C|GetbHasKey (CallFunction|GetCurrentGameInstance)
    (:then
      (Default|CallRemoveKey _gi_main)
      (Default|CallAttachButton _gi_main))
    (:else
      (Variables|Default|SetRowName "MissingKey")))
  (return (Variables|Default|GetRowName)))