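; Actor component that tracks whether the player holds a key, through a single HasKey flag on the game instance.
; On BeginPlay it clears the flag and binds events to the game instance's AddKey and RemoveKey dispatchers.
; Its AddToInventory and RemoveFromInventory events set the flag true and false, so the component stores no inventory state of its own.
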(event Custom|AddToInventory
  (Variables|/Game/Blueprint/GI_Main.GI_Main_C|SetbHasKey (CallFunction|GetCurrentGameInstance) true))

(event Custom|RemoveFromInventory
  (Variables|/Game/Blueprint/GI_Main.GI_Main_C|SetbHasKey (CallFunction|GetCurrentGameInstance) false))

(event EventBeginPlay
  (bind _gi_main (CallFunction|GetCurrentGameInstance))
  (Variables|/Game/Blueprint/GI_Main.GI_Main_C|SetbHasKey (CallFunction|GetCurrentGameInstance) false)
  (EventDispatchers|BindEventtoAddKey _gi_main (EventDispatchers|CreateEvent :!event Custom|AddToInventory))
  (EventDispatchers|BindEventtoRemoveKey _gi_main (EventDispatchers|CreateEvent :!event Custom|RemoveFromInventory)))