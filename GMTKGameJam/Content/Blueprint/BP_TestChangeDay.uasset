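; Test interactable actor that triggers a day change when the player has a key.
; Interact checks the game instance's HasKey for validity, then fires RemoveKey on it and its own ChangeDay call.
; Without a key, it returns the "MissingKey" row name to the caller.
; BeginPlay caches the first-person character, which the interaction logic does not use.
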(event EventBeginPlay
  (bind _returnvalue (Actor|GetActorOfClass "/Game/FirstPerson/Blueprints/PlayerCharacter/BP_FirstPersonCharacter.BP_FirstPersonCharacter_C"))
  (Variables|Default|SetCharacter _returnvalue))

(event Collision|EventActorBeginOverlap
  (params (OtherActor :type Actor%20Object%20Reference)))

(event EventTick
  (params (DeltaSeconds :type Float%20%28single-precision%29)))

(fn ConstructionScript)

(fn Interact
  (Variables|/Game/Blueprint/GI_Main.GI_Main_C|GetbHasKey (CallFunction|GetCurrentGameInstance)
    (:then
      (Default|CallRemoveKey (CallFunction|GetCurrentGameInstance))
      (Default|CallChangeDay))
    (:else
      (Variables|Default|SetRowName "MissingKey")))
  (return (Variables|Default|GetRowName)))