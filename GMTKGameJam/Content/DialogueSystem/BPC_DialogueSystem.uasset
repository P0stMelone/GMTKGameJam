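; Dialogue component that plays linear conversations from rows in the DT_Dialogues data table.
; StartDialogue sets the current row name, and PlayCurrentLine broadcasts that row's text through OnDialogueUpdate.
; NextLine follows each row's NextRowName like a linked list to play the following line.
; OnDialogueEnded fires when the next name is None or a row lookup in PlayCurrentLine fails.
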(event EventBeginPlay)

(event EventTick
  (params (DeltaSeconds :type Float%20%28single-precision%29)))

(fn StartDialogue
  (params (RowName :type Name))
  (Variables|Default|SetCurrentRowName RowName)
  (CallFunction|PlayCurrentLine))

(fn PlayCurrentLine
  (bind _returnvalue (Utilities|GetDataTableRow "/Game/DialogueSystem/DT_Dialogues.DT_Dialogues" (Variables|Default|GetCurrentRowName))
    (:then
      (Default|CallOnDialogueUpdate (.DialogueText (Utilities|Struct|BreakF_DialogueLine _returnvalue))))
    (:RowNotFound
      (Default|CallOnDialogueEnded))))

(fn NextLine
  (bind _returnvalue (Utilities|GetDataTableRow "/Game/DialogueSystem/DT_Dialogues.DT_Dialogues" (Variables|Default|GetCurrentRowName))
    (:then
      (if (!= (.NextRowName (Utilities|Struct|BreakF_DialogueLine _returnvalue)) "None")
        (Variables|Default|SetCurrentRowName (.NextRowName (Utilities|Struct|BreakF_DialogueLine _returnvalue)))
        (CallFunction|PlayCurrentLine)
        (else
          (Default|CallOnDialogueEnded))))))